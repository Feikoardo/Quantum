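; BP_Button_Elevator is a physical, touch-driven button that sends its floor to an elevator when pressed.
; An overlap while active records the touching component and calls ButtonTrigger, or, if already pressed, only resets that flag after a delay.
; Tick holds the button at a fixed depressed height during contact, leaving the computed press depth unused, then interpolates it back.
; SetActive toggles input and swaps the base material with a red-dot one.
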(event `self.ReceiveBeginPlay`
  (set `self.Base Material` (`|GetArrayItem` (`MeshComponent.GetMaterials` (`self.Button`))))
  (if (not (`self.IsActive`))
    (`PrimitiveComponent.SetMaterial` (`self.Button`) 0 "/Game/Materials/M_RedDot.M_RedDot")))

(event `ButtonPress`
  (`/Game/Blueprints/BP_Elevator.ButtonTrigger` (`self.Elevator`) (`self.Floor`)))

(event `self.Button.OnComponentBeginOverlap`
  (params (OverlappedComponent :type "PrimitiveComponent Object Reference") (OtherActor :type "Actor Object Reference") (OtherComp :type "PrimitiveComponent Object Reference") (OtherBodyIndex :type Integer) (bFromSweep :type Boolean) (SweepResult :type "HitResult Structure (by ref)"))
  (if (`self.IsActive`)
    (`/Engine/EditorBlueprintResources/StandardMacros.IsValid` (`self.Overlapped component`)
      (:`Is Not Valid`
        (bind _output_get (set `self.Overlapped component` OtherComp))
        (set `self.InitialOverlapLocation` (`SceneComponent.K2_GetComponentLocation` _output_get))
        (if (`self.ButtonPressed`)
          (`KismetSystemLibrary.PrintString` "Delayed")
          (`KismetSystemLibrary.Delay` 0.5)
          (set `self.ButtonPressed` false)
          (else
            (`self.ButtonPress`)
            (set `self.ButtonPressed` true)))))))

(event `self.Base.OnComponentEndOverlap`
  (params (OverlappedComponent :type "PrimitiveComponent Object Reference") (OtherActor :type "Actor Object Reference") (OtherComp :type "PrimitiveComponent Object Reference") (OtherBodyIndex :type Integer))
  (if (== (stale `self.Button.OnComponentEndOverlap` OtherComp) (`self.Overlapped component`)) :!label _label
    (set `self.Overlapped component` null)))

(event `self.Button.OnComponentEndOverlap`
  (params (OverlappedComponent :type "PrimitiveComponent Object Reference") (OtherActor :type "Actor Object Reference") (OtherComp :type "PrimitiveComponent Object Reference") (OtherBodyIndex :type Integer))
  (goto _label))

(event `self.ReceiveTick`
  (params (DeltaSeconds :type "Float (single-precision)"))
  (bind _button (`self.Button`))
  (bind _base (`self.Base`))
  (bind (_returnvalue_x _returnvalue_y _returnvalue_z) (`KismetMathLibrary.BreakVector` (- (`KismetMathLibrary.InverseTransformLocation` (`SceneComponent.K2_GetComponentToWorld` _base) (`self.InitialOverlapLocation`)) (`KismetMathLibrary.InverseTransformLocation` (`SceneComponent.K2_GetComponentToWorld` _base) (`SceneComponent.K2_GetComponentLocation` (`self.Overlapped component`))))))
  (`|ExecutionSequence`
    (:`then_0`
      (`/Engine/EditorBlueprintResources/StandardMacros.IsValid` (`self.Overlapped component`)
        (:`Is Valid`
          (bind _output_get (set `self.ButtonPressAmount` (`KismetMathLibrary.FClamp` _returnvalue_z 0.0 (`self.MaxButtonPressedAmount`))))
          (`SceneComponent.K2_SetRelativeLocation` _button (0.0 0.0 3.0) false false))
        (:`Is Not Valid`
          (`SceneComponent.K2_SetRelativeLocation` _button (`KismetMathLibrary.VInterpTo` (`SceneComponent.RelativeLocation` (`self.Button`)) (0.0 0.0 6.0) DeltaSeconds) false false))))))

(fn `SetActive`
  (params (InActive :type Boolean))
  (set `self.IsActive` InActive)
  (`KismetSystemLibrary.PrintString` "Button active!")
  (if (`self.IsActive`)
    (`PrimitiveComponent.SetMaterial` (`self.Button`) 0 (`self.Base Material`))
    (else
      (`PrimitiveComponent.SetMaterial` (`self.Button`) 0 "/Game/Materials/M_RedDot.M_RedDot"))))

(fn `UserConstructionScript`)
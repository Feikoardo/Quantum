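; BP_PortalTrigger is a portal trigger that moves a VR player into its connected room.
; On overlap while active, it clears the player's CanTeleport flag, then uses a dot product to check that the capsule is on the box's forward-facing side.
; If that passes and ConnectedRoom is valid and not already current, it teleports VROrigin to that room and updates CurrentRoom, printing debug messages along the way.
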(event `self.ReceiveBeginPlay`)

(event `self.ReceiveActorBeginOverlap`
  (params (OtherActor :type "Actor Object Reference"))
  (bind _connectedroom (`self.ConnectedRoom`))
  (bind _connectedroom_2 (`self.ConnectedRoom`))
  (if (`self.IsActive`)
    (bind _asbp_player_controller (cast `/Game/Blueprints/BP_PlayerController` OtherActor))
    (if (`/Game/Blueprints/BP_PlayerController.CanTeleport` _asbp_player_controller)
      (set `/Game/Blueprints/BP_PlayerController.CanTeleport` false _asbp_player_controller)
      (bind _out (`self.EnterForward` (`SceneComponent.K2_GetComponentLocation` (`/Game/Blueprints/BP_PlayerController.Capsule` _asbp_player_controller))))
      (if _out
        (bind _out_2 (`self.IsCurrentRoom` _asbp_player_controller))
        (if (not _out_2)
          (`KismetSystemLibrary.PrintString` "Player Overlaps portal!")
          (`/Engine/EditorBlueprintResources/StandardMacros.IsValid` _connectedroom_2
            (:`Is Valid`
              (`SceneComponent.K2_SetWorldLocation` (`/Game/VirtualRealityBP/Blueprints/MotionControllerPawn.VROrigin` _asbp_player_controller) (`self.K2_GetActorLocation` _connectedroom_2) false true)
              (set `/Game/Blueprints/BP_PlayerController.CurrentRoom` _connectedroom _asbp_player_controller)
              (`KismetSystemLibrary.PrintString` (`KismetSystemLibrary.GetObjectName` _connectedroom) true true (struct :`R` 1.0 :`A` 1.0) 5.0))))))))

(fn `EnterForward`
  (params (InPlayerPos :type "Vector Structure"))
  (returns (Out :type Boolean))
  (locals (PortalToPlayer :type "Vector Structure") (DotProduct :type "Float (double-precision)"))
  (bind _output_get (set `local.PortalToPlayer` (`KismetMathLibrary.Normal` (- InPlayerPos (`SceneComponent.K2_GetComponentLocation` (`self.Box`))))))
  (`KismetSystemLibrary.PrintString` (`KismetStringLibrary.Conv_VectorToString` _output_get))
  (set `local.DotProduct` (* (`KismetMathLibrary.Dot_VectorVector` (`SceneComponent.GetForwardVector` (`self.Box`)) (`local.PortalToPlayer`)) -1.0))
  (if (< (`local.DotProduct`) 0.0)
    (`KismetSystemLibrary.PrintString` "Forward" true true (struct :`R` 0.554167 :`G` 0.023521 :`B` 0.049992 :`A` 1.0) 10.0)
    (`KismetSystemLibrary.PrintString` (`KismetStringLibrary.Conv_DoubleToString` (`local.DotProduct`)) true true (struct :`R` 1.0 :`B` 0.116805 :`A` 1.0))
    (return true)
    (else
      (`KismetSystemLibrary.PrintString` "Not frorward")
      (return false))))

(fn `IsCurrentRoom`
  (params (InOther :type "/Game/Blueprints/BP_PlayerController Object Reference"))
  (returns (Out :type Boolean))
  (bind _currentroom (`/Game/Blueprints/BP_PlayerController.CurrentRoom` InOther))
  (if (== _currentroom (`self.ConnectedRoom`))
    (`KismetSystemLibrary.PrintString` "Room Equal")
    (`KismetSystemLibrary.PrintString` (`KismetSystemLibrary.GetObjectName` _currentroom))
    (return true)
    (else
      (`KismetSystemLibrary.PrintString` "Room not Equal")
      (return false))))

(fn `UserConstructionScript`)
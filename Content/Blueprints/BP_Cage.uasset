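; BP_Cage is a cage that locks a referenced CagedObject until the cage's completion condition is met.
; On BeginPlay it turns off physics simulation on the caged object's mesh and makes it non-grabbable.
; Completion checks run through the parent class; OnComplete makes both the object and the cage grabbable when Complete is true.
; Physics on the caged object is not re-enabled here.
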(event `self.ReceiveBeginPlay`
  (bind _cagedobject (`self.CagedObject`))
  (`parent.ReceiveBeginPlay`)
  (`/Engine/EditorBlueprintResources/StandardMacros.IsValid` _cagedobject
    (:`Is Valid`
      (`PrimitiveComponent.SetSimulatePhysics` (`StaticMeshActor.StaticMeshComponent` _cagedobject) false)
      (set `/Game/VirtualRealityBP/Blueprints/BP_PickupCube.Grabable` false _cagedobject))))

(fn `CheckForComplete`
  (`parent.CheckForComplete`)
  (`self.IsCompleted`))

(fn `IsGrabable`
  (returns (IsGrabable :type Boolean))
  (return (`self.Grabable`)))

(fn `OnComplete`
  (`parent.OnComplete`)
  (`/Engine/EditorBlueprintResources/StandardMacros.IsValid` (`self.CagedObject`)
    (:`Is Valid`
      (if (`self.Complete`)
        (set `/Game/VirtualRealityBP/Blueprints/BP_PickupCube.Grabable` true (`self.CagedObject`))
        (set `self.Grabable` true)))))

(fn `UserConstructionScript`
  (`parent.UserConstructionScript`))
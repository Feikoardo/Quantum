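; BP_PuzzleBase is a base Blueprint for puzzles that belong to a room and track whether they are completed.
; SetRoom stores the owning room, and IsCompleted returns the completion flag.
; OnComplete and OnNotComplete set or clear that flag, then ask a valid room to check if it is cleared.
; ResetPuzzle is an empty stub, and debug messages print on room assignment and completion.
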(fn `IsCompleted`
  (returns (OutComleted :type Boolean))
  (return (`self.Complete`)))

(fn `OnComplete`
  (bind _room (`self.Room`))
  (`KismetSystemLibrary.PrintString` "Puzzle Completed" true true (struct :`R` 0.168218 :`G` 1.0 :`B` 0.11582 :`A` 1.0))
  (set `self.Complete` true)
  (`/Engine/EditorBlueprintResources/StandardMacros.IsValid` _room
    (:`Is Valid`
      (`/Game/Blueprints/BP_Room.CheckIfCleared` _room))))

(fn `OnNotComplete`
  (bind _room (`self.Room`))
  (set `self.Complete` false)
  (`/Engine/EditorBlueprintResources/StandardMacros.IsValid` _room
    (:`Is Valid`
      (`/Game/Blueprints/BP_Room.CheckIfCleared` _room))))

(fn `ResetPuzzle`)

(fn `SetRoom`
  (params (InRoom :type "/Game/Blueprints/BP_Room Object Reference"))
  (set `self.Room` InRoom)
  (`KismetSystemLibrary.PrintString` "Room Set!" true true (struct :`R` 0.967272 :`G` 0.210747 :`B` 1.0 :`A` 1.0)))

(fn `UserConstructionScript`)
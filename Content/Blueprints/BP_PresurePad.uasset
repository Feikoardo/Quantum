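; Weight-triggered pressure pad that detects BP_PickupSnapable objects and completes when their combined weight reaches RequiredWeight.
; Dropped pickups entering the resizable SnapBox are tracked and stopped; leaving the actor removes them.
; Snap queries expose allow and multi-snap flags, while GetSnapPoint also registers the pickup before returning the snap location.
; CheckForComplete sums the weights, swaps the cube's green or red material, and calls OnComplete or OnNotComplete.
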(event `self.ReceiveTick`
  (params (DeltaSeconds :type "Float (single-precision)")))

(event `self.ReceiveActorEndOverlap`
  (params (OtherActor :type "Actor Object Reference"))
  (bind _asbp_pickup_snapable (cast `/Game/Blueprints/BP_PickupSnapable` OtherActor))
  (`KismetArrayLibrary.Array_RemoveItem` (`self.ObjectsOnPlate`) _asbp_pickup_snapable)
  (`KismetSystemLibrary.PrintString` "Add Object")
  (`self.CheckForComplete`))

(event `self.SnapBox.OnComponentBeginOverlap`
  (params (OverlappedComponent :type "PrimitiveComponent Object Reference") (OtherActor :type "Actor Object Reference") (OtherComp :type "PrimitiveComponent Object Reference") (OtherBodyIndex :type Integer) (bFromSweep :type Boolean) (SweepResult :type "HitResult Structure (by ref)"))
  (bind _asbp_pickup_snapable (cast `/Game/Blueprints/BP_PickupSnapable` OtherActor))
  (if (`/Game/VirtualRealityBP/Blueprints/BP_PickupCube.Dropped` _asbp_pickup_snapable)
    (`KismetArrayLibrary.Array_Add` (`self.ObjectsOnPlate`) _asbp_pickup_snapable)
    (`KismetSystemLibrary.PrintString` "Add Object")
    (`PrimitiveComponent.SetPhysicsLinearVelocity` (`StaticMeshActor.StaticMeshComponent` _asbp_pickup_snapable) (0.0 0.0 0.0) false "None")
    (`self.CheckForComplete`)))

(fn `CanSnap`
  (returns (OutCanSnap :type Boolean))
  (return (`self.AllowSnap`)))

(fn `CheckForComplete`
  (locals (WeightOnPlate :type "Float (double-precision)"))
  (for _array_element (`self.ObjectsOnPlate`)
    (set `local.WeightOnPlate` (+ (`local.WeightOnPlate`) (`/Game/Blueprints/BP_PickupSnapable.Weight` _array_element))))
  (set `self.CurrentWeight` (`local.WeightOnPlate`))
  (if (>= (`local.WeightOnPlate`) (`self.RequiredWeight`))
    (`PrimitiveComponent.SetMaterial` (`self.Cube`) 0 "/Engine/EngineDebugMaterials/VertexColorViewMode_GreenOnly.VertexColorViewMode_GreenOnly")
    (`self.OnComplete`)
    (else
      (`PrimitiveComponent.SetMaterial` (`self.Cube`) 0 "/Engine/EngineDebugMaterials/VertexColorViewMode_RedOnly.VertexColorViewMode_RedOnly")
      (`self.OnNotComplete`))))

(fn `GetSnapPoint`
  (params (InSnapable :type "/Game/Blueprints/BP_PickupSnapable Object Reference"))
  (returns (OutSnapPoint :type "Vector Structure"))
  (if (not (`KismetArrayLibrary.Array_Contains` (`self.ObjectsOnPlate`) InSnapable))
    (`KismetArrayLibrary.Array_Add` (`self.ObjectsOnPlate`) InSnapable))
  (`self.CheckForComplete`)
  (return (`SceneComponent.K2_GetComponentLocation` (`self.SnapPoint`))))

(fn `MultipleSnaps`
  (returns (Out :type Boolean))
  (return (`self.AllowMultiSnap`)))

(fn `UserConstructionScript`
  (`SceneComponent.SetWorldScale3D` (`self.SnapBox`) (`self.TriggerSize`)))
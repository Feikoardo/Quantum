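; BP_Room is a puzzle room that tracks completion of its puzzles and controls its teleports and elevator button.
; On BeginPlay it registers itself with each puzzle and closes teleports, which only happens when OnCompleteTeleportActive is set.
; CheckIfCleared activates the teleports and button once all valid puzzles are complete; otherwise it deactivates the button and re-closes teleports.
; RoomCleared latches true and is never reset here.
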(event `self.ReceiveBeginPlay`
  (for _array_element (`self.Puzzles`)
    (`/Game/Blueprints/BP_PuzzleBase.SetRoom` _array_element self))
  (`self.ClosePortals`))

(fn `CheckIfCleared`
  (for _array_element (`self.Puzzles`)
    (`/Engine/EditorBlueprintResources/StandardMacros.IsValid` _array_element
      (:`Is Valid`
        (bind _outcomleted (`/Game/Blueprints/BP_PuzzleBase.IsCompleted` _array_element))
        (if (not _outcomleted)
          (`/Engine/EditorBlueprintResources/StandardMacros.IsValid` (`self.ElevatorButton`)
            (:`Is Valid`
              (`/Game/Blueprints/BP_Button_Elevator.SetActive` (`self.ElevatorButton`) false))
            (:`Is Not Valid`
              _))
          (`self.ClosePortals`)
          (return)))))
  (set `self.RoomCleared` true)
  (`self.OnClear`)
  (`/Engine/EditorBlueprintResources/StandardMacros.IsValid` (`self.ElevatorButton`)
    (:`Is Valid`
      (`/Game/Blueprints/BP_Button_Elevator.SetActive` (`self.ElevatorButton`) true))
    (:`Is Not Valid`
      _))
  (return))

(fn `ClosePortals`
  (if (`self.OnCompleteTeleportActive`)
    (for _array_element (`self.Teleports`)
      (set `/Game/Blueprints/BP_PortalTrigger.IsActive` false _array_element))))

(fn `IsCleared`
  (returns (IsCleared :type Boolean))
  (return (`self.RoomCleared`)))

(fn `OnClear`
  (for _array_element (`self.Teleports`)
    (set `/Game/Blueprints/BP_PortalTrigger.IsActive` true _array_element))
  (`KismetSystemLibrary.PrintString` "Room is Cleared" true true (struct :`G` 1.0 :`B` 0.178869 :`A` 1.0) 5.0))

(fn `UserConstructionScript`)
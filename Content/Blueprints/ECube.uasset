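; ECube is a cube actor that can be entangled and exposes functions for grabbing or pickup.
; Entangle turns gravity off on its static mesh and Untangle restores it, both only while the mesh simulates physics.
; IsGrabable and GetStaticMesh expose the grab flag and mesh.
; CanReachPosition runs a debug-drawn visibility trace, succeeding when nothing is hit or the hit actor implements PickupActorInterface.
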(event `self.ReceiveBeginPlay`)

(event `/Game/Blueprints/I_Entangalable.Entangle`
  (if (`SceneComponent.IsSimulatingPhysics` (`self.StaticMeshComponent`) "None")
    (`PrimitiveComponent.SetEnableGravity` (`self.StaticMeshComponent`) false)))

(event `/Game/Blueprints/I_Entangalable.Untangle`
  (if (`SceneComponent.IsSimulatingPhysics` (`self.StaticMeshComponent`) "None")
    (`PrimitiveComponent.SetEnableGravity` (`self.StaticMeshComponent`) true)))

(fn `CanReachPosition`
  (params (TraceStart :type "Vector Structure") (TraceEnd :type "Vector Structure"))
  (returns (CanBeReached :type Boolean))
  (locals (Reach :type Boolean))
  (bind (_outhit _returnvalue) (`KismetSystemLibrary.LineTraceSingle` :`Start` TraceStart :`End` TraceEnd :`TraceChannel` "TraceTypeQuery1" :`DrawDebugType` "ForDuration" :`DrawTime` 0.25))
  (if _returnvalue
    (set `local.Reach` (`KismetSystemLibrary.DoesImplementInterface` (`.HitActor` (`GameplayStatics.BreakHitResult` _outhit)) "/Game/VirtualRealityBP/Blueprints/PickupActorInterface.PickupActorInterface_C"))
    (else
      (set `local.Reach` true)))
  (return (`local.Reach`)))

(fn `GetStaticMesh`
  (returns (`Static Mesh Component` :type "StaticMeshComponent Object Reference"))
  (return (`self.StaticMeshComponent`)))

(fn `IsGrabable`
  (returns (IsGrabable :type Boolean))
  (return (`self.Grabable`)))

(fn `UserConstructionScript`)
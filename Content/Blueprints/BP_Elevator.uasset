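; BP_Elevator is a VR elevator that carries the player vertically to the room passed in by a button trigger.
; A trigger while the player overlaps the collider starts a timeline that lerps the platform to that room's height, at a distance-scaled play rate.
; Buttons follow using stored height offsets, and Tick matches the VR origin's height to the platform.
; On arrival, the player's VR origin teleports to the room and CurrentRoom updates.
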(event `self.ReceiveBeginPlay`
  ;[1 1 1] Set start & end loc based on end_point and start_point components
  (`|ExecutionSequence`
    (:`then_0`
      (set `self.StartLoc` (`SceneComponent.K2_GetComponentLocation` (`self.Start`)))
      (set `self.EndLoc` (`SceneComponent.RelativeLocation` (`self.End`))))
    (:`then_1`
      ;[1 1 1] Set offset between button height and elevator floor height
      (bind _output_get (set `self.newLocation` (`SceneComponent.K2_GetComponentLocation` (`self.Elevator`))))
      (for _array_element (`self.Button`)
        (bind (_returnvalue_x _returnvalue_y _returnvalue_z) (`KismetMathLibrary.BreakVector` (`SceneComponent.K2_GetComponentLocation` (`/Game/Blueprints/BP_Button_Elevator.DefaultSceneRoot` _array_element))))
        (`BlueprintMapLibrary.Map_Add` (`self.ButtonLocation`) _array_element (- _returnvalue_z (.z _output_get)))))))

(event `ButtonTrigger`
  (params (InNewEnd :type "/Game/Blueprints/BP_Room Object Reference"))
  (bind _newroom (`self.NewRoom`))
  (bind (_startloc_x _startloc_y) (`KismetMathLibrary.BreakVector` (`self.StartLoc`)))
  (bind _playercontroller (`self.PlayerController`))
  (bind (_returnvalue_x _returnvalue_y _returnvalue_z) (`KismetMathLibrary.BreakVector` (`SceneComponent.K2_GetComponentLocation` (`/Game/Blueprints/BP_Room.DefaultSceneRoot` InNewEnd))))
  (if (`self.OnElevator`)
    (if (not (`self.ElevatorMoves`))
      (set `self.NewRoom` InNewEnd)
      (set `self.EndLoc` (`KismetMathLibrary.MakeVector` _startloc_x _startloc_y _returnvalue_z))
      (set `self.ElevatorMoves` true)
      ;[1 1 1] Set speed & delay
      (bind _output_get (set `self.MovementSpeedVar` (/ (`self.MovementSpeed`) (`KismetMathLibrary.VSize` (- (`SceneComponent.K2_GetComponentLocation` (`self.Start`)) (`SceneComponent.K2_GetComponentLocation` (`self.End`)))))))
      (`TimelineComponent.SetPlayRate` (`self.Timeline_0`) _output_get)
      (`KismetSystemLibrary.Delay` (`self.Delay`))
      ;[1 1 1] Set relative location based on timeline
      (bind (_direction _newtrack_0) (`Timeline|Timeline_0` :!via `PlayFromStart` :!label _label)
        (:`Update`
          (bind _returnvalue (`KismetMathLibrary.VLerp` (`self.StartLoc`) (`self.EndLoc`) _newtrack_0))
          (set `self.newLocation` _returnvalue)
          (`SceneComponent.K2_SetWorldLocation` (`self.Elevator`) _returnvalue false false)
          (`|ExecutionSequence`
            (:`then_0`
              (for _array_element (`self.Button`)
                (bind (_relativelocation_x _relativelocation_y) (`KismetMathLibrary.BreakVector` (`SceneComponent.RelativeLocation` (`/Game/Blueprints/BP_Button_Elevator.DefaultSceneRoot` _array_element))))
                (`self.K2_SetActorRelativeLocation` _array_element (`KismetMathLibrary.MakeVector` _relativelocation_x _relativelocation_y (+ (.z (stale _output_get_2)) (`BlueprintMapLibrary.Map_Find` (`self.ButtonLocation`) _array_element))) false false)))
            (:`then_1`
              (bind _output_get_2 (set `self.newLocation` (`SceneComponent.K2_GetComponentLocation` (`self.Elevator`)))))))
        (:`Finished`
          (set `self.StartLoc` (`self.EndLoc`))
          (set `self.ElevatorMoves` false)
          (`SceneComponent.K2_SetWorldLocation` (`/Game/VirtualRealityBP/Blueprints/MotionControllerPawn.VROrigin` _playercontroller) (`SceneComponent.K2_GetComponentLocation` (`Actor.RootComponent` _newroom)) false true)
          (set `/Game/Blueprints/BP_PlayerController.CurrentRoom` _newroom _playercontroller))))))

(event `StopPlatform`
  ;[1 1 1] Simply stops platform when this function is called
  (goto _label :!via `Stop`))

(event `self.Collider.OnComponentBeginOverlap`
  (params (OverlappedComponent :type "PrimitiveComponent Object Reference") (OtherActor :type "Actor Object Reference") (OtherComp :type "PrimitiveComponent Object Reference") (OtherBodyIndex :type Integer) (bFromSweep :type Boolean) (SweepResult :type "HitResult Structure (by ref)"))
  (bind _asbp_player_controller (cast `/Game/Blueprints/BP_PlayerController` OtherActor))
  (bind _output_get (set `self.PlayerController` _asbp_player_controller))
  (set `self.newLocation` (`SceneComponent.K2_GetComponentLocation` (`/Game/VirtualRealityBP/Blueprints/MotionControllerPawn.VROrigin` _output_get)))
  (set `self.OnElevator` true))

(event `self.Collider.OnComponentEndOverlap`
  (params (OverlappedComponent :type "PrimitiveComponent Object Reference") (OtherActor :type "Actor Object Reference") (OtherComp :type "PrimitiveComponent Object Reference") (OtherBodyIndex :type Integer))
  (bind _asbp_player_controller (cast `/Game/Blueprints/BP_PlayerController` OtherActor))
  (set `self.PlayerController` _asbp_player_controller)
  (set `self.OnElevator` false))

(event `self.ReceiveTick`
  (params (DeltaSeconds :type "Float (single-precision)"))
  (bind (_newlocation_x _newlocation_y _newlocation_z) (`KismetMathLibrary.BreakVector` (`self.newLocation`)))
  (bind _vrorigin (`/Game/VirtualRealityBP/Blueprints/MotionControllerPawn.VROrigin` (`self.PlayerController`)))
  (bind (_returnvalue_x _returnvalue_y) (`KismetMathLibrary.BreakVector` (`SceneComponent.K2_GetComponentLocation` _vrorigin)))
  (if (`self.OnElevator`)
    (`SceneComponent.K2_SetWorldLocation` _vrorigin (`KismetMathLibrary.MakeVector` _returnvalue_x _returnvalue_y _newlocation_z) false false)))

(fn `UserConstructionScript`)
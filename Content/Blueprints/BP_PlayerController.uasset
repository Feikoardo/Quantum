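; BP_PlayerController tracks the player's overlap with BP_PortalTrigger actors and maintains the flags that gate portal teleporting.
; Entering a trigger sets IsOverlapping; leaving while CanTeleport is false waits briefly, then clears IsOverlapping and re-enables CanTeleport.
; The teleport itself is not performed in this graph.
; Tick also prints the capsule's world location as debug output, throttled by a Delay.
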(event `self.ReceiveTick`
  (params (DeltaSeconds :type "Float (single-precision)"))
  (`parent.ReceiveTick` DeltaSeconds)
  (`KismetSystemLibrary.Delay` 2.5)
  (`KismetSystemLibrary.PrintString` (`KismetStringLibrary.Conv_VectorToString` (`SceneComponent.K2_GetComponentLocation` (`self.Capsule`))) true true (struct :`R` 0.976017 :`G` 1.0 :`B` 0.176957 :`A` 1.0) 1.5))

(event `self.ReceiveActorEndOverlap`
  (params (OtherActor :type "Actor Object Reference"))
  (cast `/Game/Blueprints/BP_PortalTrigger` OtherActor)
  (if (not (`self.CanTeleport`))
    (`KismetSystemLibrary.Delay` 0.2)
    (if (`self.IsOverlapping`)
      (set `self.IsOverlapping` false))
    (set `self.CanTeleport` true)))

(event `self.ReceiveActorBeginOverlap`
  (params (OtherActor :type "Actor Object Reference"))
  (cast `/Game/Blueprints/BP_PortalTrigger` OtherActor)
  (set `self.IsOverlapping` true))

(fn `UserConstructionScript`
  (`parent.UserConstructionScript`))
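; Pickup actor that snaps its mesh onto a snap target when dropped.
; It remembers the latest overlapped actor implementing BP_ISnapable and clears it when that overlap ends.
; OnDrop runs the parent logic, then asks the target whether it can snap and for a snap point.
; The mesh teleports to that point, or matches only its height if the target allows multiple snaps.
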(event `self.ReceiveActorBeginOverlap`
  (params (OtherActor :type "Actor Object Reference"))
  (cast `/Game/Blueprints/BP_ISnapable` OtherActor)
  (set `self.Snapable` OtherActor))

(event `self.ReceiveActorEndOverlap`
  (params (OtherActor :type "Actor Object Reference"))
  (if (== OtherActor (`self.Snapable`))
    (set `self.Snapable` null)))

(fn `OnDrop`
  (bind _staticmeshcomponent (`self.StaticMeshComponent`))
  (bind _snapable (`self.Snapable`))
  (bind (_returnvalue_x _returnvalue_y) (`KismetMathLibrary.BreakVector` (`SceneComponent.K2_GetComponentLocation` _staticmeshcomponent)))
  (`parent.OnDrop`)
  (`/Engine/EditorBlueprintResources/StandardMacros.IsValid` _snapable
    (:`Is Valid`
      (bind _asbp_isnapable (cast `/Game/Blueprints/BP_ISnapable` _snapable))
      (bind _outcansnap (`/Game/Blueprints/BP_ISnapable.CanSnap` _asbp_isnapable))
      (if _outcansnap
        (bind _outsnappoint (`/Game/Blueprints/BP_ISnapable.GetSnapPoint` _asbp_isnapable self))
        (bind _out (`/Game/Blueprints/BP_ISnapable.MultipleSnaps` _asbp_isnapable))
        (if _out
          (`SceneComponent.K2_SetWorldLocation` _staticmeshcomponent (`KismetMathLibrary.MakeVector` _returnvalue_x _returnvalue_y (.z _outsnappoint)) false true)
          (else
            (`SceneComponent.K2_SetWorldLocation` (`self.StaticMeshComponent`) (`KismetMathLibrary.MakeVector` (.x _outsnappoint) (.y _outsnappoint) (.z _outsnappoint)) false true)))))))

(fn `UserConstructionScript`
  (`parent.UserConstructionScript`))
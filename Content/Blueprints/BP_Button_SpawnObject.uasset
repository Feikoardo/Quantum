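; A physical push button that, when touched, spawns two snapable sphere pickups at its spawn locations and triggers a linked door.
; The first overlapping component fires the press and is tracked until it leaves the Base, with a short cooldown that is also cleared on exit.
; Tick sinks the button by that component's clamped downward movement in Base space, then interpolates it back once nothing is tracked.
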(event `ButtonPress`
  (`|SpawnActorFromClass` "/Game/Blueprints/BP_PickupSnapable_Sphere.BP_PickupSnapable_Sphere_C" (`KismetMathLibrary.Conv_VectorToTransform` (`SceneComponent.K2_GetComponentLocation` (`self.SpawnLocation1`))) "Undefined" "OverrideRootScale" null null)
  (`|SpawnActorFromClass` "/Game/Blueprints/BP_PickupSnapable_Sphere.BP_PickupSnapable_Sphere_C" (`KismetMathLibrary.Conv_VectorToTransform` (`SceneComponent.K2_GetComponentLocation` (`self.SpawnLocation2`))) "Undefined" "OverrideRootScale" null null))

(event `self.Button.OnComponentBeginOverlap`
  (params (OverlappedComponent :type "PrimitiveComponent Object Reference") (OtherActor :type "Actor Object Reference") (OtherComp :type "PrimitiveComponent Object Reference") (OtherBodyIndex :type Integer) (bFromSweep :type Boolean) (SweepResult :type "HitResult Structure (by ref)"))
  (`/Engine/EditorBlueprintResources/StandardMacros.IsValid` (`self.Overlapped component`)
    (:`Is Not Valid`
      (bind _output_get (set `self.Overlapped component` OtherComp))
      (set `self.InitialOverlapLocation` (`SceneComponent.K2_GetComponentLocation` _output_get))
      (if (`self.ButtonTimer`)
        (`KismetSystemLibrary.PrintString` "Delayed")
        (else
          (`self.ButtonPress`)
          (`/Game/Blueprints/BP_Door.DoorTrigger` (`self.Door`))
          (set `self.ButtonTimer` true)
          (`KismetSystemLibrary.Delay` 2.0)
          (set `self.ButtonTimer` false))))))

(event `self.Base.OnComponentEndOverlap`
  (params (OverlappedComponent :type "PrimitiveComponent Object Reference") (OtherActor :type "Actor Object Reference") (OtherComp :type "PrimitiveComponent Object Reference") (OtherBodyIndex :type Integer))
  (if (== OtherComp (`self.Overlapped component`))
    (set `self.Overlapped component` null)
    (set `self.ButtonTimer` false)))

(event `self.ReceiveTick`
  (params (DeltaSeconds :type "Float (single-precision)"))
  (bind _button (`self.Button`))
  (bind _base (`self.Base`))
  (bind (_returnvalue_x _returnvalue_y _returnvalue_z) (`KismetMathLibrary.BreakVector` (- (`KismetMathLibrary.InverseTransformLocation` (`SceneComponent.K2_GetComponentToWorld` _base) (`self.InitialOverlapLocation`)) (`KismetMathLibrary.InverseTransformLocation` (`SceneComponent.K2_GetComponentToWorld` _base) (`SceneComponent.K2_GetComponentLocation` (`self.Overlapped component`))))))
  (`|ExecutionSequence`
    (:`then_0`
      (`/Engine/EditorBlueprintResources/StandardMacros.IsValid` (`self.Overlapped component`)
        (:`Is Valid`
          (bind _output_get (set `self.ButtonPressAmount` (`KismetMathLibrary.FClamp` _returnvalue_z 0.0 (`self.MaxButtonPressedAmount`))))
          (`SceneComponent.K2_SetRelativeLocation` _button (`KismetMathLibrary.MakeVector` 0.0 0.0 (* _output_get -1.0)) false false))
        (:`Is Not Valid`
          (`SceneComponent.K2_SetRelativeLocation` _button (`KismetMathLibrary.VInterpTo` (`SceneComponent.RelativeLocation` (`self.Button`)) (0.0 0.0 0.0) DeltaSeconds) false false))))))

(fn `UserConstructionScript`)